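; BP_Bouton is a button Blueprint meant to respond to motion controllers, apparently an unfinished exercise.
; An overlap on DetectionMotionController links the controller, storing its component and starting relative location.
; Each Tick calls CalculDelta when the linked controller differs from that stored location, or RetourInit when unlinked.
; Both functions are empty stubs, and nothing clears the link or updates the stored location outside the overlap.
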(event OnComponentBeginOverlap(DetectionMotionController)
  (params (OverlappedComponent :type Primitive%20Component%20Object%20Reference) (OtherActor :type Actor%20Object%20Reference) (OtherComp :type Primitive%20Component%20Object%20Reference) (OtherBodyIndex :type Integer) (bFromSweep :type Boolean) (SweepResult :type Hit%20Result%20Structure%20%28by%20ref%29))
  (bind _asmotion_controller_component (Utilities|Casting|CastToMotionControllerComponent OtherComp))
  (Variables|Default|SetIsLinked true)
  (bind _output_get (Variables|Default|SetHeldMC _asmotion_controller_component))
  (Variables|Default|SetOldPos (Variables|/Script/Engine.SceneComponent|GetRelativeLocation _output_get)))

(event EventTick
  (params (DeltaSeconds :type Float%20%28single-precision%29))
  (if (Variables|Default|GetIsLinked)
    (if (not (Utilities|Operators|EqualEqual (Variables|Default|GetOldPos) (Variables|/Script/Engine.SceneComponent|GetRelativeLocation (Variables|Default|GetHeldMC)) 0.0))
      (CallFunction|CalculDelta "0, 0, 0"))
    (else
      (CallFunction|RetourInit))))

(fn ConstructionScript)

(fn CalculDelta
  (params (PosInitial :type Vector) (MCref :type Motion%20Controller%20Component%20Object%20Reference))
  (return "0, 0, 0"))

(fn RetourInit)